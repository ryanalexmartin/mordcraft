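; MordCraft toolbox equipment that lets a player place Minecraft-style dirt blocks in Mordhau.
; Each late tick it previews the selected object, using a camera trace offset along the hit normal and snapped to a 100-unit grid.
; Firing respects a cooldown, finds an existing chunk by sphere overlap, then calls ServerRequestPlant so that chunk creates the block.
; Chunk creation and block-type selection are unimplemented, and debug messages go to chat.
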(event Custom|Request%20Plant
  (params (Location :type Vector) (BlockType :type Integer) (chunkToCreateOn :type Chunk%20Object%20Reference))
  (bind _returnvalue (Utilities|GetDisplayName chunkToCreateOn))
  (bind _returnvalue_2 (Utilities|String|StringToName _returnvalue))
  (bind _returnvalue_3 (Utilities|String|BuildString(Name) "" "CURRENT CHUNK: " _returnvalue_2 ""))
  (bind _returnvalue_4 (Utilities|String|BuildString(Name) _returnvalue_3 "" "Location of block we tried to create: " ""))
  (bind _returnvalue_5 (Utilities|String|BuildString(Vector) _returnvalue_4 "" Location))
  ;[1 1 1] New functionality for creating blocks
  (CallFunction|MordhauLogger (Utilities|String|ToString(Vector) Location))
  (Default|ServerCreateDirtBlock chunkToCreateOn Location chunkToCreateOn)
  ;;[1 1 1] Debug -- placement
  (bind _asbp_mordhau_player_controller (Utilities|Casting|CastToBP_MordhauPlayerController (Game|GetPlayerController 0)))
  (Default|RequestChatMessage _asbp_mordhau_player_controller _returnvalue_5 false)
  (Development|PrintString _returnvalue_5))

(event Custom|Server%20Request%20Plant
  (params (Location :type Vector) (BlockType :type Integer) (chunkToCreateOn :type Chunk%20Object%20Reference))
  (CallFunction|RequestPlant Location BlockType chunkToCreateOn))

(event EventBeginPlay)

(event EventUpdateEquipmentState
  (|CallParentFunction)
  (CallFunction|DestroyMeshPreview))

(event EventLocalPlayerLateTick
  (params (DeltaTime :type Float%20%28single-precision%29))
  (bind _returnvalue (Class|MordhauEquipment|GetParentCharacter))
  (bind _returnvalue_2 (Class|MordhauEquipment|GetAmmo))
  (bind _previewmeshcomponent (Variables|Default|GetPreviewMeshComponent))
  (bind _spawnableobjects (Variables|Default|GetSpawnableObjects))
  (bind _objecttype (Variables|Default|GetObjectType))
  (bind _output (Utilities|Array|Get(acopy) _spawnableobjects _objecttype))
  (bind (_preview _previewskeletal _cost _rotationoffset _rotationoffsetpreview _scalepreview) (Utilities|Struct|BreakBP_ToolBoxSpawnable _output))
  (bind _returnvalue_3 (< _returnvalue_2 _cost))
  (if (or (<= (Utilities|Time|GetTimeSeconds) (Variables|Default|GetNextAvailableTime)) _returnvalue_3)
    (CallFunction|DestroyMeshPreview)
    (if _returnvalue_3
      (CallFunction|CycleObjectType))
    (else
      (Utilities|IsValid _preview
        (:Is%20Valid
          (CallFunction|AddStaticMeshPreviewifNone _preview))
        (:Is%20Not%20Valid
          (Utilities|IsValid _previewskeletal
            (:Is%20Valid
              (CallFunction|AddSkeletalMeshPreviewifNone _previewskeletal)))))
      (bind (_succeeded _location _rotation) (CallFunction|ValidateSpot (Transformation|GetActorLocation _returnvalue) (Variables|/Script/Mordhau.MordhauCharacter|GetCameraRotation1P _returnvalue) "0, 0, 0"))
      (Transformation|SetWorldTransform _previewmeshcomponent (Math|Transform|MakeTransform _location (Math|Rotator|CombineRotators _rotationoffsetpreview _rotation) _scalepreview) false false)
      (Rendering|Material|SetScalarParameterValueonMaterials _previewmeshcomponent "Valid" (Math|Conversions|ToFloat(Boolean) _succeeded)))))

(event Collision|EventActorBeginOverlap
  (params (OtherActor :type Actor%20Object%20Reference)))

(event EventTick
  (params (DeltaSeconds :type Float%20%28single-precision%29)))

(fn ConstructionScript
  (|CallParentFunction))

(fn ValidateSpot
  (params (PlanterLocation :type Vector :default "0, 0, 0") (CameraRotation1P :type Rotator :default "0, 0, 0") (Offset :type Vector :default "0, 0, 0"))
  (bind _returnvalue (Game|GetPlayerCharacter 0))
  (bind _outlocation (Actor|GetActorEyesViewPoint _returnvalue))
  (bind _outhit (Collision|LineTraceByChannel _outlocation (+ _outlocation (* (Math|Vector|GetForwardVector (Variables|/Script/Engine.Actor|GetRootComponent (Game|GetPlayerCameraManager 0))) 1e+03)) "TraceTypeQuery1" false 0 "None" true "(R=1.000000,G=0.000000,B=0.000000,A=1.000000)" "(R=0.000000,G=1.000000,B=0.000000,A=1.000000)" 1.0))
  (if (== (Utilities|GetClass (.HitComponent (Collision|BreakHitResult _outhit))) "/Script/Engine.HierarchicalInstancedStaticMeshComponent")
    (Variables|Default|SetisValid true :!label _label)
    (elif (== (Utilities|GetClass (.HitComponent (Collision|BreakHitResult _outhit))) "/Script/Engine.StaticMeshComponent")
      (goto _label)
      (else
        (Variables|Default|SetisValid false))))
  (return (Variables|Default|GetisValid) (Math|Vector|MakeVector (Math|Float|SnapToGrid(Float) (.X (Math|Vector|BreakVector (+ (* (.ImpactNormal (Collision|BreakHitResult _outhit)) 5.0) (.Location (Collision|BreakHitResult _outhit))))) 1e+02) (Math|Float|SnapToGrid(Float) (.Y (Math|Vector|BreakVector (+ (* (.ImpactNormal (Collision|BreakHitResult _outhit)) 5.0) (.Location (Collision|BreakHitResult _outhit))))) 1e+02) (Math|Float|SnapToGrid(Float) (.Z (Math|Vector|BreakVector (+ (* (.ImpactNormal (Collision|BreakHitResult _outhit)) 5.0) (.Location (Collision|BreakHitResult _outhit))))) 1e+02)) "0, 0, 0" 0))

(fn FindCurrentChunkorCreateNew
  (params (CreateLocation :type Vector))
  (bind _outactors (Collision|SphereOverlapActors CreateLocation 0.0 (Utilities|Array|MakeArray "ObjectTypeQuery1") "/Game/Mordhau/Maps/MordCraft/Chunk_Old.Chunk_Old_C"))
  (bind _aschunk (Utilities|Casting|CastToChunk (Utilities|Array|Get(acopy) _outactors))
    (:then
      (bind _output_get (Variables|Default|SetCurrent%20Chunk _aschunk))
      (CallFunction|MordhauLogger (Utilities|String|BuildString(Name) "" "" "Set current chunk to: " (Utilities|GetDisplayName _output_get)))
      (return _output_get CreateLocation 1))
    (:CastFailed
      (CallFunction|MordhauLogger "cast to chunk failed"))))

(fn MordhauLogger
  (params (InputString :type String))
  (bind _asbp_mordhau_player_controller (Utilities|Casting|CastToBP_MordhauPlayerController (Game|GetPlayerController 0)))
  (Default|RequestChatMessage _asbp_mordhau_player_controller InputString false)
  (Development|PrintString "Hello"))

(fn OnRequestFire
  (params (Character :type Mordhau%20Character%20Object%20Reference))
  (bind _returnvalue (Utilities|Time|GetTimeSeconds))
  (if (> _returnvalue (Variables|Default|GetNextAvailableTime))
    (bind (_succeeded _location) (CallFunction|ValidateSpot "0, 0, 0" "0, 0, 0" "0, 0, 0"))
    (if _succeeded
      (Variables|Default|SetNextAvailableTime (+ _returnvalue (Variables|Default|GetCooldown)))
      (CallFunction|MordhauLogger "Requested plant, validating spot...")
      (bind (_current_chunk _out_location _blocktype) (CallFunction|FindCurrentChunkorCreateNew _location))
      (CallFunction|ServerRequestPlant _out_location _blocktype _current_chunk)
      (return false))))