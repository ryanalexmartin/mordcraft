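; Metal shovel weapon for the MordCraft map, an unfinished prototype for digging blocks out of voxel chunks.
; Its Box overlap takes the hit HISM instance's world location, finds a Chunk via a small sphere overlap, and calls ServerRequestDeleteBlock.
; That event and its passthrough are empty stubs, so nothing is deleted here.
; Attack events toggle IsSwinging, which the overlap ignores; a debug logger writes to chat and screen.
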(event OnComponentBeginOverlap(Box)
  (params (OverlappedComponent :type Primitive%20Component%20Object%20Reference) (OtherActor :type Actor%20Object%20Reference) (OtherComp :type Primitive%20Component%20Object%20Reference) (OtherBodyIndex :type Integer) (bFromSweep :type Boolean) (SweepResult :type Hit%20Result%20Structure%20%28by%20ref%29))
  (bind _ashierarchical_instanced_static_mesh_component (Utilities|Casting|CastToHierarchicalInstancedStaticMeshComponent OtherComp))
  (bind _outactors (Collision|SphereOverlapActors (Transformation|GetActorLocation OtherActor) 0.2 (Utilities|Array|MakeArray "ObjectTypeQuery1") "/Game/Mordhau/Maps/MordCraft/Chunk.Chunk_C"))
  (bind _aschunk (Utilities|Casting|CastToChunk (Utilities|Array|Get(acopy) _outactors)))
  (CallFunction|ServerRequestDeleteBlock _aschunk _ashierarchical_instanced_static_mesh_component 0 (Math|Transform|TransformLocation (.OutInstanceTransform (Components|InstancedStaticMesh|GetInstanceTransform _ashierarchical_instanced_static_mesh_component OtherBodyIndex true)) "0, 0, 0")))

(event Custom|ServerRequestDeleteBlock
  (params (Target%20Chunk :type Chunk%20Object%20Reference) (ISM%20Type :type Instanced%20Static%20Mesh%20Component%20Object%20Reference) (Index :type Integer) (Location :type Vector))
  ;[1 1 1] Chunk should handle deletion...
)

(event Custom|Server%20Print
  (CallFunction|MordhauLogger "Server event was called!"))

(event EventBeginPlay
  (|CallParentFunction)
  (Actor|GetAllActorsOfClass "/Game/Mordhau/Blueprints/Characters/BP_MordhauCharacter.BP_MordhauCharacter_C")
  (Actor|SetOwner 0))

(event EventOnAttackStarted
  (params (Move :type EAttackMove%20Enum :default "RightStrike") (Angle :type Float%20%28single-precision%29))
  (Variables|Default|SetisSwinging true))

(event EventOnAttackStopped
  (Variables|Default|SetisSwinging false))

(event EventStartThrownTrail)

(fn ConstructionScript
  (|CallParentFunction))

(fn MordhauLogger
  (params (Message :type String))
  (bind _asbp_mordhau_player_controller (Utilities|Casting|CastToBP_MordhauPlayerController (Game|GetPlayerController 0)))
  (Default|RequestChatMessage _asbp_mordhau_player_controller Message false)
  (Development|PrintString Message))

(fn PassthroughRequestDeleteBlock
  (params (Target :type %20Object%20Reference) (ISM%20Type :type Instanced%20Static%20Mesh%20Component%20Object%20Reference) (Index :type Integer) (Location :type Vector)))